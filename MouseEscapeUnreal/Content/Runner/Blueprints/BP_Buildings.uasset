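; BP_Buildings is an endless-runner floor segment that populates itself with randomly placed obstacles.
; Its construction script builds spawn points along each lane, shuffles them and attaches one to three child actors, randomly choosing between two branches.
; Any overlap with its Box tells BP_RunnerGameMode to extend the floor, then slightly raises the player's walk speed within a clamped range and prints it.
; GetAttachPoint exposes the Arrow's world transform.
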(event OnComponentBeginOverlap(Box)
  (params (OverlappedComponent :type Primitive%20Component%20Object%20Reference) (OtherActor :type Actor%20Object%20Reference) (OtherComp :type Primitive%20Component%20Object%20Reference) (OtherBodyIndex :type Integer) (bFromSweep :type Boolean) (SweepResult :type Hit%20Result%20Structure%20%28by%20ref%29))
  ;[0.15 0.15 0.15 0.5] Extend Floor
  (bind _asbp_runner_game_mode (Utilities|Casting|CastToBP_RunnerGameMode (Game|GetGameMode)))
  (Default|ExtendFloor _asbp_runner_game_mode)
  ;[0.15 0.15 0.15 0.5] Change Speed
  (bind _asbp_runner_character (Utilities|Casting|CastToBP_RunnerCharacter (Game|GetPlayerCharacter 0)))
  (bind _output_get (Variables|/Script/Engine.CharacterMovementComponent|SetMaxWalkSpeed (Variables|/Script/Engine.Character|GetCharacterMovement _asbp_runner_character) (Math|Float|Clamp(Float) (* (Variables|/Script/Engine.CharacterMovementComponent|GetMaxWalkSpeed (Variables|/Script/Engine.Character|GetCharacterMovement _asbp_runner_character)) 1.001) 7e+02 1.5e+03)))
  (Development|PrintString (Utilities|String|ToString(Float) _output_get)))

(event EventBeginPlay)

(event Collision|EventActorBeginOverlap
  (params (OtherActor :type Actor%20Object%20Reference)))

(event EventTick
  (params (DeltaSeconds :type Float%20%28single-precision%29)))

(fn ConstructionScript
  (CallFunction|SetupSpawnPoints)
  (CallFunction|SpawnObstacles))

(fn GetAttachPoint
  (return (Transformation|GetWorldTransform (Variables|Default|GetArrow))))

(fn SetupSpawnPoints
  (for _array_element (Variables|Components|GetLane%20Position)
    (for _index (range 0 1)
      (bind _returnvalue (AddComponent|AddArrowComponent false (Math|Transform|MakeTransform (Math|Vector|MakeVector (* _index 6.5e+02) _array_element 0.0))))
      (Utilities|Array|Add (Variables|Default|GetSpawn%20Points) (Transformation|GetWorldTransform _returnvalue)))))

(fn SpawnObstacles
  (bind _output_get (LocalVariables|SetRandom%20Spawn%20Points (Variables|Default|GetSpawn%20Points)))
  (Utilities|Array|Shuffle _output_get)
  (for _index (range 0 (Math|Random|RandomIntegerinRange 0 2))
    (switch int (Math|Random|RandomIntegerinRange 0 1)
      (:0
        (AddComponent|AddChildActorComponent false (Math|Transform|MakeRelativeTransform (Utilities|Array|Get(acopy) (LocalVariables|GetRandom%20Spawn%20Points) _index) (Transformation|GetActorTransform))))
      (:1
        (AddComponent|AddChildActorComponent false (Math|Transform|MakeRelativeTransform (Utilities|Array|Get(acopy) (LocalVariables|GetRandom%20Spawn%20Points) _index) (Transformation|GetActorTransform)))))))